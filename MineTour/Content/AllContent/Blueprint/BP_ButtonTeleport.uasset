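; BP_ButtonTeleport is a clickable widget button that moves the player from one panorama sphere to a linked one.
; On BeginPlay it creates a WBP_TeleporterButton for its widget component and binds the click to TeleportPlayer.
; A timeline then switches panorama opacity outright from CurrentSphere to SphereLink, while lerping the character from its current location toward the linked TPPoint with sweep and teleport.
; The player position stored at BeginPlay is unused here.
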(event Custom|TeleportPlayer
  (bind _time (Timeline|Timeline Play)
    (:Update
      (Rendering|Material|SetScalarParameterValueonMaterials (Variables|/Game/AllContent/Blueprint/BP_Panorama.BP_Panorama_C|Getpanorama (Variables|Default|GetSphereLink)) "OpacityValue" 1.0)
      (Rendering|Material|SetScalarParameterValueonMaterials (Variables|/Game/AllContent/Blueprint/BP_Panorama.BP_Panorama_C|Getpanorama (Variables|Default|GetcurrentSphere)) "OpacityValue" 0.0)
      (Transformation|SetActorLocation (Game|GetPlayerCharacter 0) (Math|Vector|Lerp(Vector) (Transformation|GetWorldLocation (Variables|/Script/Engine.Actor|GetRootComponent (Game|GetPlayerCharacter 0))) (Transformation|GetWorldLocation (Variables|/Game/AllContent/Blueprint/BP_Panorama.BP_Panorama_C|GetTP_Point (Variables|Default|GetSphereLink))) _time) true true))))

(event EventBeginPlay
  (bind _returnvalue (Game|ConstructObjectfromClass (Variables|Default|GetButtonTeleport) "/Game/AllContent/UI/WBP_TeleporterButton.WBP_TeleporterButton_C"))
  (bind _output_get (Variables|Default|SetWidget _returnvalue))
  (UserInterface|SetWidget (Variables|Default|GetButtonTeleport) _output_get)
  (Variables|Default|SetCurrentPlayerPosition (Transformation|GetActorLocation (Game|GetPlayerController 0)))
  (EventDispatchers|BindEventtoOnClicked (Variables|/Game/AllContent/UI/WBP_TeleporterButton.WBP_TeleporterButton_C|GetTeleportButton (.AsWBP%20Teleporter%20Button (Utilities|Casting|CastToWBP_TeleporterButton (UserInterface|GetWidget (Variables|Default|GetButtonTeleport))))) (delegate Custom|TeleportPlayer)))

(fn ConstructionScript)